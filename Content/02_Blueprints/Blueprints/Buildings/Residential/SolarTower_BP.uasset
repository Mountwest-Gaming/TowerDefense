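; SolarTower_BP is a Solar Tower building that fires projectiles at a target.
; BeginPlay loads its stats from the tower data table, and Tick fires TowerProjectile_BP at any valid target with the configured damage, throttled by a fire-rate delay and reload flag.
; SpawnonClick spawns a Minion at the referenced building's horizontal position.
; The Knight_BP target-assignment logic is disconnected, so nothing here sets the target.
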(event `Spawn on Click`
  (params (BuildingRef :type "Actor Object Reference"))
  (bind (_returnvalue_x _returnvalue_y) (`KismetMathLibrary.BreakVector` (`self.K2_GetActorLocation` BuildingRef)))
  (`|SpawnActorFromClass` "/Game/02_Blueprints/Blueprints/Minion.Minion_C" (`KismetMathLibrary.MakeTransform` (`KismetMathLibrary.MakeVector` _returnvalue_x _returnvalue_y 10.0)) "Undefined" "OverrideRootScale" null null))

(event `self.ReceiveTick`
  (params (DeltaSeconds :type "Float (single-precision)"))
  (`/Engine/EditorBlueprintResources/StandardMacros.IsValid` (`self.TowerTarget`)
    (:`Is Valid`
      (if (not (`self.Reload`))
        (`self.Shoot`)))))

(event `Shoot`
  (bind (_damage _range _firerate) (break `/Game/02_Blueprints/TowerStruct` (`self.TowerStruct`)))
  (set `self.Reload` true)
  (`|SpawnActorFromClass` "/Game/02_Blueprints/Blueprints/Buildings/TowerProjectile_BP.TowerProjectile_BP_C" (`self.GetTransform`) "Undefined" "OverrideRootScale" null (`self.TowerTarget`) _damage null)
  (`KismetSystemLibrary.Delay` _firerate)
  (set `self.Reload` false))

(event `self.ReceiveBeginPlay`
  (bind _returnvalue (`|GetDataTableRow` "/Game/02_Blueprints/TowerDataTable.TowerDataTable" "SolarTower")
    (:`then`
      (set `self.TowerStruct` _returnvalue))))

(fn `UserConstructionScript`
  (`parent.UserConstructionScript`))