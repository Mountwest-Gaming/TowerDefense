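; Tower projectile that homes on a TargetRunner actor and damages it on overlap.
; Tick moves it at constant speed toward the runner, caching that location so it keeps flying there if the runner becomes invalid.
; The overlap applies damage only to the target and leaves the projectile alive.
; Destruction occurs only in the invalid-target branch, whose proximity check reads the invalid runner's location instead of the cached one.
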(event `self.ReceiveTick`
  (params (DeltaSeconds :type "Float (single-precision)"))
  (bind _targetrunner (`self.TargetRunner`))
  (bind _projectile_speed (`self.Projectile Speed`))
  (bind _returnvalue (`self.K2_GetActorLocation` _targetrunner))
  (`/Engine/EditorBlueprintResources/StandardMacros.IsValid` _targetrunner
    (:`Is Valid`
      (set `self.LastKnownLoc` _returnvalue)
      (`self.K2_SetActorLocation` (`KismetMathLibrary.VInterpTo_Constant` (`self.K2_GetActorLocation`) _returnvalue DeltaSeconds _projectile_speed)))
    (:`Is Not Valid`
      (if (< (`KismetMathLibrary.VSize` (- (`self.K2_GetActorLocation`) (`self.K2_GetActorLocation` _targetrunner))) 20.0)
        (`self.K2_DestroyActor`)
        (else
          (`self.K2_SetActorLocation` (`KismetMathLibrary.VInterpTo_Constant` (`self.K2_GetActorLocation`) (`self.LastKnownLoc`) DeltaSeconds _projectile_speed)))))))

(event `self.Collision.OnComponentBeginOverlap`
  (params (OverlappedComponent :type "PrimitiveComponent Object Reference") (OtherActor :type "Actor Object Reference") (OtherComp :type "PrimitiveComponent Object Reference") (OtherBodyIndex :type Integer) (bFromSweep :type Boolean) (SweepResult :type "HitResult Structure (by ref)"))
  (bind _targetrunner (`self.TargetRunner`))
  (if (== OtherActor _targetrunner)
    (`GameplayStatics.ApplyDamage` _targetrunner (`self.Damage`))))

(fn `UserConstructionScript`)