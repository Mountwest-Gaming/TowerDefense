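; Knight enemy that walks to the tower and detonates on contact.
; On BeginPlay it takes the tower reference from GameModePog, then issues an AI MoveTo toward it every Tick while valid.
; Overlapping the tower subtracts Damage from TowerHealth, runs the tower's death check, spawns an explosion emitter and destroys the knight.
; Incoming damage lowers Health and destroys the knight at zero or below.
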(event `self.ReceiveBeginPlay`
  ;[1 1 1] Begin Play
  (bind _asgame_mode_pog (cast `/Game/02_Blueprints/GameBPs/GameModePog` (`GameplayStatics.GetGameMode`)))
  (set `self.TowerRef` (`/Game/02_Blueprints/GameBPs/GameModePog.Tower Ref` _asgame_mode_pog)))

(event `self.ReceiveActorBeginOverlap`
  (params (OtherActor :type "Actor Object Reference"))
  (bind _towerref (`self.TowerRef`))
  (if (== OtherActor _towerref)
    (set `/Game/02_Blueprints/Tower_BP.TowerHealth` (- (`/Game/02_Blueprints/Tower_BP.TowerHealth` _towerref) (`self.Damage`)) _towerref)
    (`/Game/02_Blueprints/Tower_BP.CheckForDeath` (`self.TowerRef`))
    (`GameplayStatics.SpawnEmitterAtLocation` "/Game/09_VFX/Explosion.Explosion" (`SceneComponent.K2_GetComponentLocation` (`self.CapsuleComponent`)))
    (`self.K2_DestroyActor`)))

(event `self.ReceiveTick`
  (params (DeltaSeconds :type "Float (single-precision)"))
  ;[1 1 1 1 10] Called every frame
  ; Avoid if at all possible
  ;[1 1 1 1 10] Get validated Tower Ref
  (bind _towerref (`self.TowerRef`)
    (:`then`
      ;[1 1 1 1 10] Move to Tower Reference
      (`|AIMoveTo` self (0.0 0.0 0.0) _towerref 10.0))
    (:`else`)))

(event `self.ReceiveAnyDamage`
  (params (Damage :type "Float (single-precision)") (DamageType :type "DamageType Object Reference") (InstigatedBy :type "Controller Object Reference") (DamageCauser :type "Actor Object Reference"))
  (set `self.Health` (- (`self.Health`) Damage))
  (if (<= (`self.Health`) 0.0)
    (`self.K2_DestroyActor`)))

(fn `UserConstructionScript`)